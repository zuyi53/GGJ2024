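; Throwable grenade actor that explodes on impact and raises a laugh count when it hits an AI character.
; Sphere hits count only while Throw is set, spawning a short-lived BP_Explosion and destroying the grenade.
; A hit on BP_ALSAI calls IncreaseLaugh on the cached GGJGameStateBase.
; The construction script picks a random mesh from the Mesh array, never selecting the last of multiple entries.
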(event OnComponentHit(Sphere)
  (params (HitComponent :type Primitive%20Component%20Object%20Reference) (OtherActor :type Actor%20Object%20Reference) (OtherComp :type Primitive%20Component%20Object%20Reference) (NormalImpulse :type Vector :default "0, 0, 0") (Hit :type Hit%20Result%20Structure%20%28by%20ref%29))
  (if (Variables|Default|GetbThrow?)
    (CallFunction|Explosion)
    (Utilities|Casting|CastToBP_ALSAI OtherActor)
    (Default|IncreaseLaugh (Variables|Default|GetAs%20GGJGame%20State%20Base))
    (Development|PrintString "increase")))

(event Custom|Explosion
  (Development|PrintString (Utilities|String|ToString(Vector) (.Location (Collision|BreakHitResult (stale OnComponentHit(Sphere) Hit)))))
  (bind _returnvalue (Game|SpawnActorfromClass "/Game/Core/BP_Explosion.BP_Explosion_C" (Transformation|GetActorTransform) "Undefined" "OverrideRootScale" 0 0))
  (Actor|SetLifeSpan _returnvalue 3.0)
  (Actor|DestroyActor))

(event EventBeginPlay
  (bind _asggjgame_state_base (Utilities|Casting|CastToGGJGameStateBase (Game|GetGameState)))
  (Variables|Default|SetAs%20GGJGame%20State%20Base _asggjgame_state_base))

(fn ConstructionScript
  (bind _mesh (Variables|Default|Getmesh))
  (Components|StaticMesh|SetStaticMesh (Variables|Default|GetStaticMesh) (Utilities|Array|Get(acopy) _mesh (Math|Random|RandomInteger (- (Utilities|Array|Length _mesh) 1)))))