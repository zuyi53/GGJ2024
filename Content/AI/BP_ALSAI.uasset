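; BP_ALSAI is an AI actor with a capsule component that can raise a temporary shield and reacts audibly to grenade hits.
; Sheild_On spawns a BP_Sheild at the SpawnPoint transform, then destroys it after a short delay.
; Capsule hits from an exact BP_Grenade class play a 2D damage sound, with no health or damage logic in this graph.
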(event OnComponentHit(CapsuleComponent)
  (params (HitComponent :type Primitive%20Component%20Object%20Reference) (OtherActor :type Actor%20Object%20Reference) (OtherComp :type Primitive%20Component%20Object%20Reference) (NormalImpulse :type Vector :default "0, 0, 0") (Hit :type Hit%20Result%20Structure%20%28by%20ref%29))
  (if (== (Utilities|GetClass OtherActor) "/Game/Core/BP_Grenade.BP_Grenade_C")
    (Audio|PlaySound2D "/Game/sound/SC_Damaged.SC_Damaged" 1.0 1.0 0.0 0 0)))

(event Custom|Sheild_On
  (bind _returnvalue (Game|SpawnActorfromClass "/Game/AI/BTs/BP_Sheild.BP_Sheild_C" (Transformation|GetWorldTransform (Variables|Default|GetSpawn_Point)) "AlwaysSpawn" "MultiplyWithRoot" 0 0))
  (Utilities|FlowControl|Delay 2.5)
  (Actor|DestroyActor _returnvalue))

(event EventBeginPlay
  (|CallParentFunction) ; This node is disabled and will not be called.\nDrag off pins to build functionality.
)

(event Collision|EventActorBeginOverlap
  (params (OtherActor :type Actor%20Object%20Reference)))

(event EventTick
  (params (DeltaSeconds :type Float%20%28single-precision%29))
  (|CallParentFunction DeltaSeconds) ; This node is disabled and will not be called.\nDrag off pins to build functionality.
)

(fn ConstructionScript
  (|CallParentFunction))