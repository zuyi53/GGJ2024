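; Grenade actor that explodes on impact once it has been thrown.
; A hit on its Sphere component triggers the Explosion event only when the Throw flag is set.
; Explosion prints the hit location, spawns a short-lived BP_Explosion at the grenade's transform, then destroys the grenade.
; A BP_Boss cast leading to the same explosion is left disconnected and never runs.
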(event OnComponentHit(Sphere)
  (params (HitComponent :type Primitive%20Component%20Object%20Reference) (OtherActor :type Actor%20Object%20Reference) (OtherComp :type Primitive%20Component%20Object%20Reference) (NormalImpulse :type Vector :default "0, 0, 0") (Hit :type Hit%20Result%20Structure%20%28by%20ref%29))
  (if (Variables|Default|GetbThrow?)
    (CallFunction|Explosion)))

(event Custom|Explosion
  (Development|PrintString (Utilities|String|ToString(Vector) (.Location (Collision|BreakHitResult (stale OnComponentHit(Sphere) Hit)))))
  (bind _returnvalue (Game|SpawnActorfromClass "/Game/BP/BP_Explosion.BP_Explosion_C" (Transformation|GetActorTransform) "Undefined" "OverrideRootScale" 0 0))
  (Actor|SetLifeSpan _returnvalue 3.0)
  (Actor|DestroyActor))

(fn ConstructionScript)